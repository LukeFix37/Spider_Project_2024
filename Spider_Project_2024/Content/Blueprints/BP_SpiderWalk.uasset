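; BP_SpiderWalk animates a Spider component through a repeating walk-and-turn cycle that starts on BeginPlay.
; A movement timeline adds a lerped step to the spider's relative X each update, so movement accumulates rather than following absolute positions.
; SpiderRot plays a second timeline that accumulates yaw with roll and pitch fixed, triggered shortly after each walk starts and again when it finishes, before the delayed loop.
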(event `self.ReceiveBeginPlay`
  (`|ExecutionSequence` :!label _label
    (:`then_0`
      (bind (_direction _newtrack_0) (`Timeline|Timeline_3` :!via `PlayFromStart`)
        (:`Update`
          (`SceneComponent.K2_SetRelativeLocation` (`self.Spider`) (`KismetMathLibrary.MakeVector` (+ (.x (`SceneComponent.RelativeLocation` (`self.Spider`))) (`KismetMathLibrary.Lerp` (`self.A_0`) (`self.B_0`) _newtrack_0)) (.y (`SceneComponent.RelativeLocation` (`self.Spider`))) (.z (`SceneComponent.RelativeLocation` (`self.Spider`)))) false false))
        (:`Finished`
          (`self.SpiderRot`)
          (`KismetSystemLibrary.Delay` 1.0)
          (goto _label))))
    (:`then_1`
      (`KismetSystemLibrary.Delay` 1.0)
      (`self.SpiderRot`))))

(event `SpiderRot`
  (bind (_direction _spiderrot) (`Timeline|Rot` :!via `PlayFromStart`)
    (:`Update`
      (`SceneComponent.K2_SetRelativeRotation` (`self.Spider`) (`KismetMathLibrary.MakeRotator` 90.0 0.0 (+ (.yaw (`SceneComponent.RelativeRotation` (`self.Spider`))) _spiderrot)) false false))))

(fn `UserConstructionScript`)